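; BP_Guard is an enemy guard that roams at random and reacts when it sees a pawn.
; Wander loops AI moves to random reachable points around the midpoint between the guard and world origin, biasing it toward center, with random pauses between moves.
; On sight, it stops, focuses on the pawn for a second, prints a life-loss message without applying damage, then resumes wandering.
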(event `self.PawnSensing.OnSeePawn`
  (params (Pawn :type "Pawn Object Reference"))
  (bind _returnvalue (`AIBlueprintHelperLibrary.GetAIController` self))
  (set `self.bIsStaring` true)
  (`Controller.StopMovement` _returnvalue)
  (`AIController.K2_SetFocus` _returnvalue Pawn)
  (`KismetSystemLibrary.Delay` 1.0)
  (`KismetSystemLibrary.PrintText` "PLAYER DETECTED -1 TO LIFE FORCES")
  (set `self.bIsStaring` false)
  (`AIController.K2_ClearFocus` _returnvalue)
  (`self.Wander`))

(event `self.ReceiveBeginPlay`
  (`self.Wander`))

(event `Wander`
  (if (not (`self.bIsStaring`))
    (`|AIMoveTo` self (`NavigationSystemV1.K2_GetRandomReachablePointInRadius` (`KismetMathLibrary.VLerp` (`self.K2_GetActorLocation`) (0.0 0.0 0.0) 0.5) 1000.0 null null) null
      (:`OnSuccess`
        _)
      (:`OnFail`
        _))
    (`KismetSystemLibrary.Delay` (`KismetMathLibrary.RandomFloatInRange` 0.1 5.0))
    (`self.Wander`)))

(fn `UserConstructionScript`)