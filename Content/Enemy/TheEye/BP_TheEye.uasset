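; BP_TheEye is an enemy eye that looks around at random and damages the player on contact with its cone.
; From BeginPlay, a self-calling Look event eases the Sphere to a random pitch and yaw, pauses briefly, then repeats.
; When the Cone component begins overlapping a BP_PlayerChar, it applies a fixed amount of damage once per overlap.
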(event `Look`
  (`KismetSystemLibrary.MoveComponentTo` (`self.Sphere`) (0.0 0.0 0.0) (`KismetMathLibrary.MakeRotator` 0.0 (`KismetMathLibrary.RandomFloatInRange` -60.0 60.0) (`KismetMathLibrary.RandomFloatInRange` -60.0 60.0)) true true 3.0)
  (`KismetSystemLibrary.Delay` 1.0)
  (`self.Look`))

(event `self.ReceiveBeginPlay`
  (`self.Look`))

(event `self.Cone.OnComponentBeginOverlap`
  (params (OverlappedComponent :type "PrimitiveComponent Object Reference") (OtherActor :type "Actor Object Reference") (OtherComp :type "PrimitiveComponent Object Reference") (OtherBodyIndex :type Integer) (bFromSweep :type Boolean) (SweepResult :type "HitResult Structure (by ref)"))
  (bind _asbp_player_char (cast `/Game/Player/BP_PlayerChar` OtherActor))
  (`GameplayStatics.ApplyDamage` _asbp_player_char 30.0))

(fn `UserConstructionScript`)